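; BP_OstPlayer is an actor that plays a random soundtrack track when the game begins.
; On BeginPlay it picks a random entry from SoundList, assigns it to its AudioComponent, lowers the volume multiplier and starts playback.
; It picks only once, with no logic to switch tracks afterward.
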(event EventBeginPlay
  (bind _audiocomponent (Variables|Components|GetAudioComponent))
  (Audio|Components|Audio|SetSound (Variables|Components|GetAudioComponent) (Utilities|Array|Get(acopy) (Variables|Default|GetSoundList) (Math|Random|RandomIntegerinRange 0 (- (Utilities|Array|Length (Variables|Default|GetSoundList)) 1))))
  (Audio|Components|Audio|SetVolumeMultiplier _audiocomponent 0.05 :!class /Script/Engine.AudioComponent)
  (Audio|Components|Audio|Play _audiocomponent 0.0))

(fn ConstructionScript)