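; Hover component that keeps its owner's physics-simulated root body floating above surfaces beneath it.
; BeginPlay caches the root primitive only if it simulates physics.
; Each tick it traces down along world up, ignoring the owner, and converts the hit distance into normalized compression.
; A spring-damper, using stiffness plus damping on compression change since the last hit, applies force along the component's up vector at its location.
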(event EventBeginPlay
  ;[0.0625 0.0625 0.0625] Begin Play (Check for physics simulation)
  (bind _asprimitive_component (Utilities|Casting|CastToPrimitiveComponent (Variables|/Script/Engine.Actor|GetRootComponent (Components|GetOwner))))
  (bind _output_get (Variables|Default|SetBody%20Ref _asprimitive_component))
  (if (not (Physics|IsSimulatingPhysics _output_get "None"))
    (Variables|Default|SetBody%20Ref 0)))

(event EventTick
  (params (DeltaSeconds :type Float%20%28single-precision%29))
  (bind _returnvalue (Transformation|GetWorldLocation))
  (bind _distance_between_hover_to_ground (Variables|Default|GetDistance%20Between%20Hover%20to%20Ground))
  (Variables|Default|GetBody%20Ref
    (:then
      (bind (_outhit _returnvalue_2) (Collision|LineTraceByChannel _returnvalue (- _returnvalue (* (Math|Vector|GetUpVector "0, 0, 0") (Variables|Default|GetDistance%20Between%20Hover%20to%20Ground))) "TraceTypeQuery1" false (Utilities|Array|MakeArray (Components|GetOwner)) "None"))
      (if _returnvalue_2
        (Variables|Default|SetHover%20Force (+ (* (/ (- (/ (- _distance_between_hover_to_ground (.Distance (Collision|BreakHitResult _outhit))) _distance_between_hover_to_ground) (Variables|Default|GetReduce%20Compression)) (Utilities|Time|GetWorldDeltaSeconds)) (Variables|Default|GetDamping)) (* (/ (- _distance_between_hover_to_ground (.Distance (Collision|BreakHitResult _outhit))) _distance_between_hover_to_ground) (Variables|Default|GetStiffness))))
        (Variables|Default|SetReduce%20Compression (/ (- _distance_between_hover_to_ground (.Distance (Collision|BreakHitResult _outhit))) _distance_between_hover_to_ground))
        (Class|PrimitiveComponent|AddForceatLocation (Variables|Default|GetBody%20Ref) (* (Math|Vector|GetUpVector) (Variables|Default|GetHover%20Force)) (Transformation|GetWorldLocation) "None")))
    (:else)))