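; AI guard that turns toward sensed BPIPlayer pawns, fires projectiles and breaks destructible objects.
; PawnSensing drives shooting, gated by CanShoot and a Tick cooldown, though nothing here sets CanShoot true.
; Dead stops sensing, ragdolls the mesh with an impulse and asks its spawner to check zone clearance.
; Capsule hits on "Destruct" actors spawn a Chaos field and radial impulse, disabling capsule collision when debris simulates physics.
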(event OnSeePawn(PawnSensing)
  (params (Pawn :type Pawn%20Object%20Reference))
  (bind _returnvalue (Transformation|GetActorLocation))
  (bind _returnvalue_2 (Transformation|GetActorLocation Pawn))
  (bind _returnvalue_3 (Math|Rotator|FindLookatRotation _returnvalue _returnvalue_2))
  ;[1 1 1] AI Behavior
  (if (Utilities|DoesObjectImplementInterface Pawn "/Game/02-Class/03-interface/BPI-Player.BPI-Player_C")
    (Transformation|SetActorRotation (Math|Rotator|MakeRotator (.roll _returnvalue_3) 0.0 (.yaw _returnvalue_3)))
    (if (Variables|Default|GetCanShoot)
      (Game|SpawnActorfromClass "/Game/FirstPerson/Blueprints/BP_FirstPersonProjectile.BP_FirstPersonProjectile_C" (Transformation|GetWorldTransform (Variables|Default|GetArrow)) "Undefined" "MultiplyWithRoot" 0 0)
      (Variables|Default|SetActiveCooldown (Variables|Default|GetDuration))
      (Variables|Default|SetCanShoot false))))

(event OnComponentHit(Capsule)
  (params (HitComponent :type Primitive%20Component%20Object%20Reference) (OtherActor :type Actor%20Object%20Reference) (OtherComp :type Primitive%20Component%20Object%20Reference) (NormalImpulse :type Vector :default "0, 0, 0") (Hit :type Hit%20Result%20Structure%20%28by%20ref%29))
  ;[1 1 1] Casse mur
  (if (Actor|ActorHasTag OtherActor "Destruct")
    (Variables|Default|SetOther%20Actor OtherActor)
    (bind _returnvalue (Game|SpawnActorfromClass "/Engine/EditorResources/FieldNodes/FS_MasterField.FS_MasterField_C" (Math|Conversions|ToTransform(Vector) (.location Hit)) "Undefined" "MultiplyWithRoot" 0 0))
    (Variables|/Engine/EditorResources/FieldNodes/FS_MasterField.FS_MasterField_C|SetActivationType _returnvalue "NewEnumerator4")
    (Components|Sphere|SetSphereRadius (Variables|/Engine/EditorResources/FieldNodes/FS_MasterField.FS_MasterField_C|GetSphereVolumeCol _returnvalue) 1e+02 true)
    (Default|CETrigger _returnvalue)
    (bind _result (Math|Float|NegateFloat (* (Variables|Default|GetStrength%20Scale) (Variables|/Game/ChaosStrength.ChaosStrength_C|GetStength (Actor|GetComponentbyClass (Variables|Default|GetOther%20Actor) "/Game/ChaosStrength.ChaosStrength_C"))))
      (:%20%20
        (Class|PhysicsObjectBlueprintLibrary|ApplyRadialImpulse OtherComp (Transformation|GetActorLocation (Variables|Default|GetOther%20Actor)) (* (Variables|Default|GetRadius) (Variables|Default|GetRadius%20Scale)) _result "RIF_Constant" false 0.0 false 0.0 1.0)
        (if (Class|SceneComponent|IsAnySimulatingPhysics OtherComp)
          (Collision|SetCollisionObjectType OtherComp "ECC_GameTraceChannel2")
          (Collision|SetCollisionProfileName (Variables|Default|GetCapsule) "NoCollision" true :!class /Script/Engine.PrimitiveComponent))))))

(event Custom|Dead
  (params (Impulse :type Vector))
  (bind _skeletalmesh (Variables|Default|GetSkeletalMesh))
  ;[1 1 1] Ragdoll
  (Class|PawnSensingComponent|SetSensingUpdatesEnabled (Variables|Default|GetPawnSensing) false)
  (Collision|SetCollisionProfileName _skeletalmesh "Ragdoll" true :!class /Script/Engine.PrimitiveComponent)
  (Physics|SetSimulatePhysics _skeletalmesh true)
  (Physics|AddImpulse (Variables|Default|GetSkeletalMesh) Impulse "None" false)
  (Default|CheckifZoneCleared (Variables|Default|GetSpawner%20Ref)))

(event Custom|AddSpawnerRef
  (params (SpawnerRef :type BP%20Enemy%20Spawner%20Object%20Reference))
  ;[1 1 1] Setup
  (Variables|Default|SetSpawner%20Ref SpawnerRef))

(event EventTick
  (params (DeltaSeconds :type Float%20%28single-precision%29))
  ;[1 1 1] Fire Rate
  (Variables|Default|SetActiveCooldown (- (Variables|Default|GetActiveCooldown) DeltaSeconds))
  (if (<= (- (Variables|Default|GetActiveCooldown) DeltaSeconds) 0.0)
    (Variables|Default|SetCanShoot false)))

(event EventBeginPlay
  ;[1 1 1] Setup
  (Variables|Default|SetActiveCooldown (Variables|Default|GetDuration)))

(fn ConstructionScript)