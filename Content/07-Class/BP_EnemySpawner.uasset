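; Enemy spawner that populates a zone with BP_Guard actors and tracks whether it has been cleared.
; On BeginPlay, while active, it spawns one guard at each spawn point, passes itself to the guard, lists it and increments an alive count.
; CheckIfZoneCleared decrements that count and deactivates the spawner at zero.
; The loop over previously spawned guards does nothing, as its DestroyActor node is unwired.
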(event Custom|Spawn
  ;[1 1 1] Spawn Ennemy
  (if (Variables|Default|GetIsActive)
    (for _array_element (Variables|Default|GetEnnemySpawnListe)
      _)
    (for _array_element_2 (Variables|Default|Getennemy%20spawn%20point)
      (bind _returnvalue (Game|SpawnActorfromClass "/Game/06-AI/BP_Guard.BP_Guard_C" (Transformation|GetActorTransform _array_element_2) "Undefined" "MultiplyWithRoot" 0 0))
      (Math|Integer|IncrementInt (Variables|Default|GetStillAlive)
        (:%20%20
          (Default|AddSpawnerRef _returnvalue self)
          (Utilities|Array|Add (Variables|Default|GetEnnemySpawnListe) _returnvalue))))))

(event Custom|CheckIfZoneCleared
  ;[1 1 1] Check If Zone Is Cleared
  (bind _result (Math|Integer|DecrementInt (Variables|Default|GetStillAlive))
    (:%20%20
      (if (<= _result 0)
        (Variables|Default|SetIsActive false)))))

(event EventBeginPlay
  ;[1 1 1] Spawn Ennemy
  (CallFunction|Spawn))

(fn ConstructionScript)